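; BP_Class_Selection is a gameplay element that opens the class selection screen and can show an outline highlight.
; Its ClassScreeSelection event creates the UI_ClassSelect widget, adds it to the viewport, shows the mouse cursor and sets Game and UI input mode.
; ActiveOverlay and ActiveOverlayOut set and clear an outline overlay material on the static mesh.
; Nothing in this Blueprint calls these events itself.
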(event `/Game/BPI/BPI_GPE_Class_Selection.ClassScreeSelection`
  (bind _returnvalue (`GameplayStatics.GetPlayerController` 0))
  (bind _returnvalue_2 (`|CreateWidget` "/Game/UserInterface/ClassSelection/UI_ClassSelect.UI_ClassSelect_C" _returnvalue))
  (bind _output_get (set `self.UI Class Select` _returnvalue_2))
  (`UserWidget.AddToViewport` _output_get 0)
  (set `PlayerController.bShowMouseCursor` true _returnvalue)
  (`WidgetBlueprintLibrary.SetInputMode_GameAndUIEx` _returnvalue null))

(event `/Game/BPI/BPI_GPE_Overlay.ActiveOverlay`
  (`MeshComponent.SetOverlayMaterial` (`self.StaticMesh`) "/Game/AssetsOverlay/Outline_Mat1.Outline_Mat1"))

(event `/Game/BPI/BPI_GPE_Overlay_Out.ActiveOverlayOut`
  (`MeshComponent.SetOverlayMaterial` (`self.StaticMesh`) null))

(fn `UserConstructionScript`)