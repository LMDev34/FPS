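; BP_Armory is an interactable armory furniture piece that opens the armory menu.
; Two events toggle an outline overlay material on the furniture mesh to highlight it.
; Its interaction event disables player movement, blends the view to a target actor, then creates the UI_Armory widget with UI-only input and a visible cursor.
; Restoring movement, camera and input is not handled here.
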(event `/Game/BPI/BPI_GPE_Overlay.ActiveOverlay`
  (`MeshComponent.SetOverlayMaterial` (`self.MeubleArmurerie`) "/Game/AssetsOverlay/Outline_Mat1.Outline_Mat1"))

(event `/Game/BPI/BPI_GPE_Overlay_Out.ActiveOverlayOut`
  (`MeshComponent.SetOverlayMaterial` (`self.MeubleArmurerie`) null))

(event `/Game/BPI/BPI_GPE_Armurerie.Interaction_Armurerie`
  (bind _returnvalue (`GameplayStatics.GetPlayerController` 0))
  (bind _ascharacter (cast `/Game/MainAssets/EpicContent/Blueprints/Character` (`GameplayStatics.GetPlayerCharacter` 0)))
  (`CharacterMovementComponent.DisableMovement` (`Character.CharacterMovement` _ascharacter))
  (`PlayerController.SetViewTargetWithBlend` (`GameplayStatics.GetPlayerController` 0) (`self.New View Target`) 1.0 "VTBlend_Linear" 0.0 false)
  (bind _returnvalue_2 (`|CreateWidget` "/Game/UserInterface/UI_Armory.UI_Armory_C" (`GameplayStatics.GetPlayerController` 0)))
  (bind _output_get (set `self.UI_Armory` _returnvalue_2))
  (`UserWidget.AddToViewport` _output_get 0)
  (`WidgetBlueprintLibrary.SetInputMode_UIOnlyEx` _returnvalue null)
  (set `PlayerController.bShowMouseCursor` true _returnvalue))

(fn `UserConstructionScript`)