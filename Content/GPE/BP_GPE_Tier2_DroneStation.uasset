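; Tier 2 drone station that hands the player control of the BP_SmallReaper actor in the level.
; Tier2Map flags the Player as on the map, disables its movement, starts a camera blend to the Reaper and possesses it.
; CameraViewBlendback blends to the current player pawn, then after a delay possesses it and restores walking and game-only input.
; Overlay events toggle the mesh outline; the CommanderPanel widget code is unconnected.
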(event `self.Tier2Map`
  (bind _returnvalue (`GameplayStatics.GetPlayerController` 0))
  (bind _asplayer (cast `/Game/MainAssets/EpicContent/Blueprints/Player` (`GameplayStatics.GetPlayerCharacter` 0)))
  (set `/Game/MainAssets/EpicContent/Blueprints/Player.CommanderOnMap` true _asplayer)
  (`CharacterMovementComponent.DisableMovement` (`Character.CharacterMovement` _asplayer))
  (bind _returnvalue_2 (`GameplayStatics.GetActorOfClass` "/Game/Role_Abilities/CMD_TechTree/BP_SmallReaper.BP_SmallReaper_C"))
  (`PlayerController.SetViewTargetWithBlend` _returnvalue _returnvalue_2 1.0 "VTBlend_EaseInOut" 1.0 false)
  (`Controller.Possess` _returnvalue _returnvalue_2))

(event `Camera View Blendback`
  (`PlayerController.SetViewTargetWithBlend` (`GameplayStatics.GetPlayerController` 0) (`GameplayStatics.GetPlayerPawn` 0) 1.0 "VTBlend_EaseInOut" 1.0 false)
  (`KismetSystemLibrary.Delay` 1.0)
  (set `/Game/MainAssets/EpicContent/Blueprints/Player.CommanderOnMap` false (stale `self.Tier2Map` _asplayer))
  (`Controller.Possess` (`GameplayStatics.GetPlayerController` 0) (`GameplayStatics.GetPlayerPawn` 0))
  (`CharacterMovementComponent.SetMovementMode` (`Character.CharacterMovement` (stale `self.Tier2Map` _asplayer)) "MOVE_Walking" 0)
  (`WidgetBlueprintLibrary.SetInputMode_GameOnly` (`GameplayStatics.GetPlayerController` 0)))

(event `self.ActiveOverlay`
  ;[1 1 1] Active Overlay
  (`MeshComponent.SetOverlayMaterial` (`self.StaticMesh`) "/Game/AssetsOverlay/Outline_Mat1.Outline_Mat1"))

(event `self.ActiveOverlayOut`
  ;[1 1 1] Active Overlay
  (`MeshComponent.SetOverlayMaterial` (`self.StaticMesh`) null))

(fn `UserConstructionScript`)