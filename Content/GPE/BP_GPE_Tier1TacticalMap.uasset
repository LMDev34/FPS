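; BP_GPE_Tier1TacticalMap is a gameplay actor that opens the tier 1 tactical map for the player.
; Its Tier1Map event flags the player character as CommanderOnMap and disables their movement.
; It then creates the Tier1Map widget, adds it to the viewport and switches to mouse cursor with Game and UI input.
; The file contains no logic for closing the map or restoring movement.
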(event `/Game/BPI/BPI_GPE_Tier1_MapCommander.Tier1Map`
  (bind _returnvalue (`GameplayStatics.GetPlayerController` 0))
  (bind _asplayer (cast `/Game/MainAssets/EpicContent/Blueprints/Player` (`GameplayStatics.GetPlayerCharacter` 0)))
  (set `/Game/MainAssets/EpicContent/Blueprints/Player.CommanderOnMap` true _asplayer)
  (`CharacterMovementComponent.DisableMovement` (`Character.CharacterMovement` _asplayer))
  (bind _returnvalue_2 (`|CreateWidget` "/Game/UserInterface/CommanderMap/Tier1Map.Tier1Map_C" _returnvalue))
  (bind _output_get (set `self.CmdMapTier1` _returnvalue_2))
  (`UserWidget.AddToViewport` _output_get 0)
  (set `PlayerController.bShowMouseCursor` true _returnvalue)
  (`WidgetBlueprintLibrary.SetInputMode_GameAndUIEx` _returnvalue null))

(fn `UserConstructionScript`)